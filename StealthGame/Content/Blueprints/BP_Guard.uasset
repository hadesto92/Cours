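; BP_Guard is a guard character with Idle, Suspicious and Alerted states shown through a widget.
; On state change, it updates its WBP_GuardState widget with a blank, question mark or exclamation mark status.
; It also caches its max movement speed at BeginPlay and offers an event that stores a random navigable location within a given radius of an origin.
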(event EventBeginPlay
  (Variables|Default|SetGuardMovementSpeed (Class|MovementComponent|GetMaxSpeed (Variables|Character|GetCharacterMovement))))

(event Collision|EventActorBeginOverlap
  (params (OtherActor :type Actor%20Object%20Reference)))

(event EventTick
  (params (DeltaSeconds :type Float%20%28single-precision%29)))

(event EventOnStateChanged
  (params (NewState :type EAIState%20Enum :default "Idle"))
  (bind _aswbp_guard_state (Utilities|Casting|CastToWBP_GuardState (UserInterface|GetUserWidgetObject (Variables|Default|GetWidget))))
  (Default|UpdateStatus _aswbp_guard_state (Utilities|Select :Index NewState :Idle "" :Suspicious "?" :Alerted "!")))

(event EventGetRandomLocation
  (params (Origin :type Vector :default "0, 0, 0") (Radius :type Float%20%28single-precision%29))
  (bind _randomlocation (Class|NavigationSystemV1|GetRandomLocationinNavigableRadius Origin Radius 0 0))
  (Variables|Default|SetNewGeneratedLocation _randomlocation))

(fn ConstructionScript)