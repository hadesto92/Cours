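; BP_GeneratePointTest is an actor that generates random patrol points for an AI character at BeginPlay.
; It finds a BP_AICharacter in the level, then spawns TargetPoints at random navigable locations within a fixed radius of its root.
; Each spawn result is added to the character's PatrolPoints array.
; GeneratePoint calls itself recursively, incrementing MaxPointIndex until it reaches MaxPoint.
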(event Custom|GeneratePoint
  (bind _randomlocation (Class|NavigationSystemV1|GetRandomLocationinNavigableRadius (Transformation|GetWorldLocation (Variables|Default|GetDefaultSceneRoot)) 1e+03 0 0))
  (bind _returnvalue (Game|SpawnActorfromClass "/Script/Engine.TargetPoint" (Math|Transform|MakeTransform _randomlocation "0, 0, 0" "1.000000,1.000000,1.000000") "AdjustIfPossibleButDontSpawnIfColliding" 0 0))
  (Utilities|Array|Add (Variables|/Game/Blueprints/BP_AICharacter.BP_AICharacter_C|GetPatrolPoints (Variables|Default|GetAs%20BP%20AICharacter)) _returnvalue)
  (if (not (>= (Variables|Default|GetMaxPointIndex) (Variables|Default|GetMaxPoint)))
    (Math|Integer|IncrementInt (Variables|Default|GetMaxPointIndex)
      (:%20%20
        (CallFunction|GeneratePoint)))))

(event EventBeginPlay
  (bind _returnvalue (Actor|GetActorOfClass "/Game/Blueprints/BP_AICharacter.BP_AICharacter_C"))
  (Variables|Default|SetAs%20BP%20AICharacter _returnvalue)
  (CallFunction|GeneratePoint))

(event Collision|EventActorBeginOverlap
  (params (OtherActor :type Actor%20Object%20Reference)))

(event EventTick
  (params (DeltaSeconds :type Float%20%28single-precision%29)))

(fn ConstructionScript)