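; BP_AICharacter is an AI-controlled pawn that patrols a looping route of target actors.
; On BeginPlay it uses AIMoveTo to walk to the current entry in the PatrolPoints array.
; Each successful move advances PatrolPointIndex, wrapping to zero after the last point, and calls PatrolToPoint again.
; Only the Success result is handled, so a failed move ends the patrol.
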(event Custom|PatrolToPoint
  (AI|AIMoveTo self "0, 0, 0" (Utilities|Array|Get(acopy) (Variables|Default|GetPatrolPoints) (Variables|Default|GetPatrolPointIndex)) 5.0 false
    (:OnSuccess
      (if (>= (Variables|Default|GetPatrolPointIndex) (- (Utilities|Array|Length (Variables|Default|GetPatrolPoints)) 1))
        (Variables|Default|SetPatrolPointIndex 0)
        (else
          (Math|Integer|IncrementInt (Variables|Default|GetPatrolPointIndex)
            (:%20%20
              _))))
      (CallFunction|PatroltoPoint))))

(event EventBeginPlay
  (CallFunction|PatroltoPoint))

(fn ConstructionScript)